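; Procedural planet actor that builds a terrain mesh with collision on its procedural mesh component.
; The Construction Script creates a PlanetTerrainGenerator and passes it the resolution, radius, seed and layered continental, mountain and detail settings.
; The generator's vertices, triangles, normals and tangents feed straight into the mesh section.
; BeginPlay writes a hard-coded test triangle to the same default section, replacing the generated terrain at runtime.
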(event EventBeginPlay
  (Class|ProceduralMeshComponent|CreateMeshSectionLinearColor (Variables|Default|GetPlanetProceduralMesh) 0 (Utilities|Array|MakeArray "0, 0, 0" "100.000000,0.000000,0.000000" "0.000000,100.000000,0.000000") (Utilities|Array|MakeArray 0 1 2) 0 0 0 0 0 0 0 false false))

(fn ConstructionScript
  (bind _returnvalue (Game|ConstructObjectfromClass "/Script/Andromeda.PlanetTerrainGenerator"))
  (bind _output_get (Variables|Default|SetTerrainGenerator _returnvalue))
  (Class|ProceduralMeshComponent|CreateMeshSectionLinearColor (Variables|Default|GetPlanetProceduralMesh) 0 (.OutVertices (Class|PlanetTerrainGenerator|GenerateTerrainMeshData _output_get (Variables|Default|GetResolution) (Variables|Default|GetPlanetRadius) (Variables|Default|GetPlanetSeed) (Variables|Default|GetContinentalScale) (Variables|Default|GetMountainScale) (Variables|Default|GetDetailScale) (Variables|Default|GetMountainStrength) (Variables|Default|GetDetailStrength) (Variables|Default|GetTerrainHeight))) (.OutTriangles (Class|PlanetTerrainGenerator|GenerateTerrainMeshData _output_get (Variables|Default|GetResolution) (Variables|Default|GetPlanetRadius) (Variables|Default|GetPlanetSeed) (Variables|Default|GetContinentalScale) (Variables|Default|GetMountainScale) (Variables|Default|GetDetailScale) (Variables|Default|GetMountainStrength) (Variables|Default|GetDetailStrength) (Variables|Default|GetTerrainHeight))) (.OutNormals (Class|PlanetTerrainGenerator|GenerateTerrainMeshData _output_get (Variables|Default|GetResolution) (Variables|Default|GetPlanetRadius) (Variables|Default|GetPlanetSeed) (Variables|Default|GetContinentalScale) (Variables|Default|GetMountainScale) (Variables|Default|GetDetailScale) (Variables|Default|GetMountainStrength) (Variables|Default|GetDetailStrength) (Variables|Default|GetTerrainHeight))) 0 0 0 0 0 (.OutTangents (Class|PlanetTerrainGenerator|GenerateTerrainMeshData _output_get (Variables|Default|GetResolution) (Variables|Default|GetPlanetRadius) (Variables|Default|GetPlanetSeed) (Variables|Default|GetContinentalScale) (Variables|Default|GetMountainScale) (Variables|Default|GetDetailScale) (Variables|Default|GetMountainStrength) (Variables|Default|GetDetailStrength) (Variables|Default|GetTerrainHeight))) true false))